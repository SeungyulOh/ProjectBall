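; BP_Ball is the ball actor whose physics depends on the game mode's state.
; On BeginPlay it turns gravity off on its Sphere and binds a callback to the ProjectBallGameMode state change event.
; The callback enables gravity only in the PLAY state, leaving it off during IDLE, BUILDING and END.
; A leftover velocity debug print is disconnected and never runs.
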(event `self.ReceiveBeginPlay`
  (`PrimitiveComponent.SetEnableGravity` (`self.Sphere`) false)
  (bind _asproject_ball_game_mode (cast `ProjectBallGameMode` (`GameplayStatics.GetGameMode`)))
  (add `ProjectBallGameMode.OnStateChanged` _asproject_ball_game_mode (delegate `Callback_StateChanged`)))

(event `Callback_StateChanged`
  (params (eModestate :type "EGameModeState Enum" :default "IDLE"))
  (`PrimitiveComponent.SetEnableGravity` (`self.Sphere`) (select `EGameModeState` eModestate :`PLAY` true)))

(event `self.ReceiveTick`
  (params (DeltaSeconds :type "Float (single-precision)")))

(fn `UserConstructionScript`)