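; BP_TutoPoint is an actor, apparently a tutorial point marker, with a plane whose color can switch between its original value and white.
; On BeginPlay it creates a dynamic material instance for the plane and caches its "Color" parameter as OriginColor.
; The ChangeMaterialColor event sets that parameter to the cached color or to white, depending on its OriginalColor flag.
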(event `self.ReceiveBeginPlay`
  (bind _returnvalue (`PrimitiveComponent.CreateDynamicMaterialInstance` (`self.Plane`) 0 (`PrimitiveComponent.GetMaterial` (`self.Plane`) 0) "None"))
  (bind _returnvalue_2 (`MaterialInstanceDynamic.K2_GetVectorParameterValue` _returnvalue "Color"))
  (set `self.OriginColor` _returnvalue_2)
  (`PrimitiveComponent.SetMaterial` (`self.Plane`) 0 _returnvalue))

(event `self.ChangeMaterialColor`
  (params (bOriginalColor :type Boolean))
  (bind _asmaterial_instance_dynamic (cast `MaterialInstanceDynamic` (`PrimitiveComponent.GetMaterial` (`self.Plane`) 0)))
  (`MaterialInstanceDynamic.SetVectorParameterValue` _asmaterial_instance_dynamic "Color" (select `bool` bOriginalColor :`false` (make `LinearColor` 1.0 1.0 1.0 1.0) :`true` (`self.OriginColor`))))

(fn `UserConstructionScript`)